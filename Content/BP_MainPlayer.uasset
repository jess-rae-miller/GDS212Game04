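; BP_MainPlayer is the player actor, handling movement, camera look and interaction with objects, records and notes.
; BeginPlay creates the main and record UIs, and a per-tick camera trace sets the current Interactable and toggles its prompt for the Interact action.
; Record targets are traced only when RecordInteract is pressed, with a second handler starting their interaction.
; E calls NoteMessage through BPI_HNote on overlapping BP_HNote actors.
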(event EventBeginPlay
  ;[1 1 1] Display UI
  (Utilities|FlowControl|Sequence
    (:then_0
      (bind _returnvalue (Game|ConstructObjectfromClass "/Game/MainUI.MainUI_C"))
      (UserInterface|Viewport|AddtoViewport _returnvalue 0)
      (Variables|Default|SetUI _returnvalue))
    (:then_1
      (bind _returnvalue_2 (Game|ConstructObjectfromClass "/Game/RecordUI.RecordUI_C"))
      (UserInterface|Viewport|AddtoViewport _returnvalue_2 0)
      (Variables|Default|SetRecordUI _returnvalue_2))))

(event Collision|EventActorBeginOverlap
  (params (OtherActor :type Actor%20Object%20Reference)))

(event EventTick
  (params (DeltaSeconds :type Float%20%28single-precision%29))
  (bind _camera (Variables|Default|GetCamera))
  (bind _returnvalue (Transformation|GetWorldLocation _camera))
  ;[1 1 1] Interactable Object + Text type
  (bind _outhit (Collision|LineTraceByChannel _returnvalue (+ _returnvalue (* (Math|Vector|GetForwardVector (Transformation|GetWorldRotation _camera)) 2.5e+02)) "TraceTypeQuery1" false 0 "None"))
  (bind _asinteractable (Utilities|Casting|CastToInteractable (.HitActor (Collision|BreakHitResult _outhit)))
    (:then
      (if (Variables|/Game/Interactable.Interactable_C|GetCanInteract _asinteractable)
        (Variables|Default|SetCurrentInteractable _asinteractable)
        (Default|ToggleInteractText (Variables|Default|GetUI) "Visible")
        (else
          (Variables|Default|SetCurrentInteractable 0 :!label _label)
          (Default|ToggleInteractText (Variables|Default|GetUI) "Hidden"))))
    (:CastFailed
      (goto _label))))

(event Input|ActionEvents|InputActionInteract
  (params (Key :type Key%20Structure :default "None"))
  (bind _currentinteractable (Variables|Default|GetCurrentInteractable))
  ;[1 1 1] Interactable Object + Text type
  (:Pressed
    (Utilities|IsValid _currentinteractable
      (:Is%20Valid
        (Default|BeginInteraction _currentinteractable (Variables|Default|GetUI))))))

(event Input|ActionEvents|InputActionRecordInteract
  (params (Key :type Key%20Structure :default "None"))
  (bind _camera (Variables|Default|GetCamera))
  (bind _returnvalue (Transformation|GetWorldLocation _camera))
  (:Pressed
    (bind _outhit (Collision|LineTraceByChannel _returnvalue (+ _returnvalue (* (Math|Vector|GetForwardVector (Transformation|GetWorldRotation _camera)) 2.5e+02)) "TraceTypeQuery1" false 0 "None"))
    (bind _asbp_record_interact (Utilities|Casting|CastToBP_RecordInteract (.HitActor (Collision|BreakHitResult _outhit)))
      (:then
        (if (Variables|/Game/BP_RecordInteract.BP_RecordInteract_C|GetCanInteract _asbp_record_interact)
          (Variables|Default|SetRecordCurrentInteractable _asbp_record_interact)
          (Default|ToggleRecordPromptText (Variables|Default|GetRecordUI) "Visible")
          (else
            (Variables|Default|SetRecordCurrentInteractable 0 :!label _label)
            (Default|ToggleRecordPromptText (Variables|Default|GetRecordUI) "Hidden"))))
      (:CastFailed
        (goto _label)))))

(event Input|ActionEvents|InputActionRecordInteract
  (params (Key :type Key%20Structure :default "None"))
  (bind _recordcurrentinteractable (Variables|Default|GetRecordCurrentInteractable))
  (:Pressed
    (Utilities|IsValid _recordcurrentinteractable
      (:Is%20Valid
        (Default|BeginInteraction _recordcurrentinteractable)))))

(event Input|AxisEvents|InputAxisMoveForward/Backward
  (params (AxisValue :type Float%20%28single-precision%29))
  ;[1 1 1] Movement
  (Pawn|Input|AddMovementInput (Transformation|GetActorForwardVector) AxisValue false))

(event Input|AxisEvents|InputAxisMoveLeft/Right
  (params (AxisValue :type Float%20%28single-precision%29))
  ;[1 1 1] Movement
  (Pawn|Input|AddMovementInput (Transformation|GetActorRightVector) AxisValue false))

(event Input|AxisEvents|InputAxisLookLeft/Right
  (params (AxisValue :type Float%20%28single-precision%29))
  ;[1 1 1] Camera
  (Pawn|Input|AddControllerYawInput AxisValue))

(event Input|AxisEvents|InputAxisLookUp/Down
  (params (AxisValue :type Float%20%28single-precision%29))
  ;[1 1 1] Camera
  (Pawn|Input|AddControllerPitchInput AxisValue))

(event Input|KeyboardEvents|E
  (params (Key :type Key%20Structure :default "None"))
  ;[1 1 1] Note Interaction
  ;;[0 0 0] Check box for "Execute when Paused"
  (:Pressed
    (for _array_element (Collision|GetOverlappingActors "/Game/HorrorNotes/Blueprints/BP_HNote.BP_HNote_C" :!class /Script/Engine.Actor)
      (if (Utilities|DoesObjectImplementInterface _array_element "/Game/HorrorNotes/Blueprints/BPI_HNote.BPI_HNote_C")
        (Class|BPIHNote|Note(Message) _array_element)))))

(fn ConstructionScript)
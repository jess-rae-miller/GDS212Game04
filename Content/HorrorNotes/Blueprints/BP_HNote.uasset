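; BP_HNote is a readable horror note actor that shows an interact prompt while the player is inside its sphere.
; Each Note call advances a page in the flag-selected widget style, optionally locking movement or pausing the game.
; Passing the last page or leaving the sphere closes it, restoring input and speed, then resetting or retiring the note.
; Closing also drives optional extras: level streaming, actor spawning or destruction, and sound.
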(event OnComponentEndOverlap(Sphere)
  (params (OverlappedComponent :type Primitive%20Component%20Object%20Reference) (OtherActor :type Actor%20Object%20Reference) (OtherComp :type Primitive%20Component%20Object%20Reference) (OtherBodyIndex :type Integer))
  ;[1 1 1] Remove Widgets if Player Leaves Collision
  (if (== OtherActor (Game|GetPlayerCharacter 0))
    (CallFunction|RemoveWidget)
    (Utilities|IsValid (Variables|Default|GetInteract)
      (:Is%20Valid
        (Rendering|SetVisibility (Variables|Default|GetInteract) false false)))))

(event OnComponentBeginOverlap(Sphere)
  (params (OverlappedComponent :type Primitive%20Component%20Object%20Reference) (OtherActor :type Actor%20Object%20Reference) (OtherComp :type Primitive%20Component%20Object%20Reference) (OtherBodyIndex :type Integer) (bFromSweep :type Boolean) (SweepResult :type Hit%20Result%20Structure%20%28by%20ref%29))
  ;[1 1 1] Remove Widgets if Player Leaves Collision
  (if (== OtherActor (Game|GetPlayerCharacter 0))
    (Utilities|IsValid (Variables|Default|GetInteract)
      (:Is%20Valid
        (Rendering|SetVisibility (Variables|Default|GetInteract) true false)))))

(event Custom|RemoveWidget
  (bind _interact (Variables|Default|GetInteract))
  (bind _destroy (Variables|NoteSystem|GetDestroy))
  (Utilities|FlowControl|Sequence
    (:then_0
      (Utilities|IsValid (Variables|Default|GetSimpleNote)
        (:Is%20Valid
          (Widget|RemovefromParent (Variables|Default|GetSimpleNote)))))
    (:then_1
      (Utilities|IsValid (Variables|Default|GetCenterBloodUI)
        (:Is%20Valid
          (Widget|RemovefromParent (Variables|Default|GetCenterBloodUI)))))
    (:then_2
      (Utilities|IsValid (Variables|Default|GetScrapUI)
        (:Is%20Valid
          (Widget|RemovefromParent (Variables|Default|GetScrapUI)))))
    (:then_3
      (Utilities|IsValid (Variables|Default|GetBlankUI)
        (:Is%20Valid
          (Widget|RemovefromParent (Variables|Default|GetBlankUI)))))
    (:then_4
      (Utilities|IsValid (Variables|Default|GetSideUI)
        (:Is%20Valid
          (Widget|RemovefromParent (Variables|Default|GetSideUI))))))
  (Utilities|FlowControl|Delay 0.1)
  (Input|SetInputModeGameOnly (Game|GetPlayerController 0))
  (Utilities|FlowControl|Sequence
    (:then_0
      (if (Variables|NoteSystem|GetPlayerLock)
        (Variables|/Script/Engine.CharacterMovementComponent|SetMaxWalkSpeed (Variables|/Script/Engine.Character|GetCharacterMovement (Game|GetPlayerCharacter 0)) (Variables|Default|GetMaxWalkSpeed))))
    (:then_1
      (if (not (Variables|NoteSystem|GetDoOnce?))
        (Variables|Default|SetPages -1)
        (Variables|Default|SetSideUI 0)
        (Variables|Default|SetBlankUI 0)
        (Variables|Default|SetScrapUI 0)
        (Variables|Default|SetCenterBloodUI 0)
        (Variables|Default|SetSimpleNote 0)
        (else
          (Utilities|FlowControl|Sequence
            (:then_0
              (if (Variables|NoteSystem|GetDestroySelf?)
                (Utilities|FlowControl|Delay 0.1)
                (Actor|DestroyActor)))
            (:then_1
              (Utilities|IsValid _interact
                (:Is%20Valid
                  (Components|DestroyComponent _interact))))))))
    (:then_2
      (if (Variables|NoteSystem|GetDelay%20Extras)
        (Utilities|FlowControl|Delay (Variables|NoteSystem|GetDelay%20Extras%20Time)))
      (Utilities|FlowControl|Sequence
        (:then_0
          (Game|LoadStreamLevel(byName) (Variables|NoteSystem|GetLevel%202%20Load) true)
          (Game|UnloadStreamLevel(byName) (Variables|NoteSystem|GetLevel%202%20Unload) false))
        (:then_1
          (if (Variables|NoteSystem|GetSpawn%20Actor%20Once?)
            (Utilities|FlowControl|DoOnce false
              (:Completed
                _)))
          (Game|SpawnActorfromClass (Variables|NoteSystem|GetSpawn%20in%20Actor) (Variables|NoteSystem|GetSpawn%20Location) "Undefined" 0 0))
        (:then_2
          (Utilities|IsValid _destroy
            (:Is%20Valid
              (Actor|DestroyActor _destroy))))
        (:then_3
          (if (Variables|NoteSystem|GetPlay%20Close%20Sound%20Once?)
            (Utilities|FlowControl|DoOnce false
              (:Completed
                _)))
          (Audio|PlaySound2D (Variables|NoteSystem|GetSound%20Close) 1.0 1.0 0.0 0 0))))))

(event EventBeginPlay
  ;[1 1 1] Set Players Walk Speed Hide Interact
  (Rendering|SetVisibility (Variables|Default|GetInteract) false false)
  (Utilities|FlowControl|Delay 0.5)
  (Variables|Default|SetMaxWalkSpeed (Variables|/Script/Engine.CharacterMovementComponent|GetMaxWalkSpeed (Variables|/Script/Engine.Character|GetCharacterMovement (Game|GetPlayerCharacter 0)))))

(event EventNote
  (if (Variables|NoteSystem|GetPlayerLock)
    (Input|SetInputModeGameandUI (Game|GetPlayerController 0) 0 "LockAlways" true)
    (Variables|/Script/Engine.CharacterMovementComponent|SetMaxWalkSpeed (Variables|/Script/Engine.Character|GetCharacterMovement (Game|GetPlayerCharacter 0)) 0.0))
  (Math|Integer|IncrementInt (Variables|Default|GetPages)
    (:%20%20
      (if (< (Variables|Default|GetPages) (Utilities|Array|Length (Variables|NoteSystem|GetNotes)))
        (Utilities|FlowControl|Sequence
          (:then_0
            (if (Variables|NoteStyle|GetSimple)
              (Variables|Default|GetSimpleNote
                (:then
                  _)
                (:else
                  (bind _returnvalue (UserInterface|CreateWidget "/Game/HorrorNotes/Widgets/W_HN_Simple.W_HN_Simple_C" (Game|GetPlayerController 0)))
                  (bind _output_get (Variables|Default|SetSimpleNote _returnvalue))
                  (UserInterface|Viewport|AddtoViewport _output_get 0)))
              (Rendering|Components|TextRender|SetText (Variables|/Game/HorrorNotes/Widgets/W_HN_Simple.W_HN_Simple_C|GetNote (Variables|Default|GetSimpleNote)) (Utilities|Text|ToText(String) (Utilities|Array|Get(acopy) (Variables|NoteSystem|GetNotes) (Variables|Default|GetPages))))
              (Rendering|Components|TextRender|SetText (Variables|/Game/HorrorNotes/Widgets/W_HN_Simple.W_HN_Simple_C|GetTitle (Variables|Default|GetSimpleNote)) (Variables|NoteSystem|GetTitle))
              (Rendering|Components|TextRender|SetText (Variables|/Game/HorrorNotes/Widgets/W_HN_Simple.W_HN_Simple_C|GetPageTotal (Variables|Default|GetSimpleNote)) (Utilities|Text|ToText(Integer) (Utilities|Array|Length (Variables|NoteSystem|GetNotes))))
              (Rendering|Components|TextRender|SetText (Variables|/Game/HorrorNotes/Widgets/W_HN_Simple.W_HN_Simple_C|GetPageNumber (Variables|Default|GetSimpleNote)) (Utilities|Text|ToText(Integer) (+ (Variables|Default|GetPages) 1)))
              (if (Variables|NoteSystem|GetPlay%20Open%20Sound%20Once?) :!label _label
                (Utilities|FlowControl|DoOnce false
                  (:Completed
                    _)))
              (Audio|PlaySound2D (Variables|NoteSystem|GetSound%20Open) 1.0 1.0 0.0 0 0)))
          (:then_1
            (if (Variables|NoteStyle|GetCenterBlood)
              (Variables|Default|GetCenterBloodUI
                (:then
                  _)
                (:else
                  (bind _returnvalue_2 (UserInterface|CreateWidget "/Game/HorrorNotes/Widgets/W_HN_CenterBlood.W_HN_CenterBlood_C" (Game|GetPlayerController 0)))
                  (bind _output_get_2 (Variables|Default|SetCenterBloodUI _returnvalue_2))
                  (UserInterface|Viewport|AddtoViewport _output_get_2 0)))
              (Rendering|Components|TextRender|SetText (Variables|/Game/HorrorNotes/Widgets/W_HN_CenterBlood.W_HN_CenterBlood_C|GetNote (Variables|Default|GetCenterBloodUI)) (Utilities|Text|ToText(String) (Utilities|Array|Get(acopy) (Variables|NoteSystem|GetNotes) (Variables|Default|GetPages))))
              (Rendering|Components|TextRender|SetText (Variables|/Game/HorrorNotes/Widgets/W_HN_CenterBlood.W_HN_CenterBlood_C|GetTitle (Variables|Default|GetCenterBloodUI)) (Variables|NoteSystem|GetTitle))
              (Rendering|Components|TextRender|SetText (Variables|/Game/HorrorNotes/Widgets/W_HN_CenterBlood.W_HN_CenterBlood_C|GetPageTotal (Variables|Default|GetCenterBloodUI)) (Utilities|Text|ToText(Integer) (Utilities|Array|Length (Variables|NoteSystem|GetNotes))))
              (Rendering|Components|TextRender|SetText (Variables|/Game/HorrorNotes/Widgets/W_HN_CenterBlood.W_HN_CenterBlood_C|GetPageNumber (Variables|Default|GetCenterBloodUI)) (Utilities|Text|ToText(Integer) (+ (Variables|Default|GetPages) 1)))
              (goto _label)))
          (:then_2
            (if (Variables|NoteStyle|GetScrap)
              (Variables|Default|GetScrapUI
                (:then
                  _)
                (:else
                  (bind _returnvalue_3 (UserInterface|CreateWidget "/Game/HorrorNotes/Widgets/W_HN_Scrap.W_HN_Scrap_C" (Game|GetPlayerController 0)))
                  (bind _output_get_3 (Variables|Default|SetScrapUI _returnvalue_3))
                  (UserInterface|Viewport|AddtoViewport _output_get_3 0)))
              (Rendering|Components|TextRender|SetText (Variables|/Game/HorrorNotes/Widgets/W_HN_Scrap.W_HN_Scrap_C|GetNote (Variables|Default|GetScrapUI)) (Utilities|Text|ToText(String) (Utilities|Array|Get(acopy) (Variables|NoteSystem|GetNotes) (Variables|Default|GetPages))))
              (Rendering|Components|TextRender|SetText (Variables|/Game/HorrorNotes/Widgets/W_HN_Scrap.W_HN_Scrap_C|GetTitle (Variables|Default|GetScrapUI)) (Variables|NoteSystem|GetTitle))
              (Rendering|Components|TextRender|SetText (Variables|/Game/HorrorNotes/Widgets/W_HN_Scrap.W_HN_Scrap_C|GetPageTotal (Variables|Default|GetScrapUI)) (Utilities|Text|ToText(Integer) (Utilities|Array|Length (Variables|NoteSystem|GetNotes))))
              (Rendering|Components|TextRender|SetText (Variables|/Game/HorrorNotes/Widgets/W_HN_Scrap.W_HN_Scrap_C|GetPageNumber (Variables|Default|GetScrapUI)) (Utilities|Text|ToText(Integer) (+ (Variables|Default|GetPages) 1)))
              (goto _label)))
          (:then_3
            (if (Variables|NoteStyle|GetBlank)
              (Variables|Default|GetBlankUI
                (:then
                  _)
                (:else
                  (bind _returnvalue_4 (UserInterface|CreateWidget "/Game/HorrorNotes/Widgets/W_HN_Blank.W_HN_Blank_C" (Game|GetPlayerController 0)))
                  (bind _output_get_4 (Variables|Default|SetBlankUI _returnvalue_4))
                  (UserInterface|Viewport|AddtoViewport _output_get_4 0)))
              (Rendering|Components|TextRender|SetText (Variables|/Game/HorrorNotes/Widgets/W_HN_Blank.W_HN_Blank_C|GetNote (Variables|Default|GetBlankUI)) (Utilities|Text|ToText(String) (Utilities|Array|Get(acopy) (Variables|NoteSystem|GetNotes) (Variables|Default|GetPages))))
              (Rendering|Components|TextRender|SetText (Variables|/Game/HorrorNotes/Widgets/W_HN_Blank.W_HN_Blank_C|GetTitle (Variables|Default|GetBlankUI)) (Variables|NoteSystem|GetTitle))
              (Rendering|Components|TextRender|SetText (Variables|/Game/HorrorNotes/Widgets/W_HN_Blank.W_HN_Blank_C|GetPageTotal (Variables|Default|GetBlankUI)) (Utilities|Text|ToText(Integer) (Utilities|Array|Length (Variables|NoteSystem|GetNotes))))
              (Rendering|Components|TextRender|SetText (Variables|/Game/HorrorNotes/Widgets/W_HN_Blank.W_HN_Blank_C|GetPageNumber (Variables|Default|GetBlankUI)) (Utilities|Text|ToText(Integer) (+ (Variables|Default|GetPages) 1)))
              (goto _label)))
          (:then_4
            (if (Variables|NoteStyle|GetSide)
              (Variables|Default|GetSideUI
                (:then
                  _)
                (:else
                  (bind _returnvalue_5 (UserInterface|CreateWidget "/Game/HorrorNotes/Widgets/W_HN_Side.W_HN_Side_C" (Game|GetPlayerController 0)))
                  (bind _output_get_5 (Variables|Default|SetSideUI _returnvalue_5))
                  (UserInterface|Viewport|AddtoViewport _output_get_5 0)))
              (Rendering|Components|TextRender|SetText (Variables|/Game/HorrorNotes/Widgets/W_HN_Side.W_HN_Side_C|GetNote (Variables|Default|GetSideUI)) (Utilities|Text|ToText(String) (Utilities|Array|Get(acopy) (Variables|NoteSystem|GetNotes) (Variables|Default|GetPages))))
              (Rendering|Components|TextRender|SetText (Variables|/Game/HorrorNotes/Widgets/W_HN_Side.W_HN_Side_C|GetTitle (Variables|Default|GetSideUI)) (Variables|NoteSystem|GetTitle))
              (Rendering|Components|TextRender|SetText (Variables|/Game/HorrorNotes/Widgets/W_HN_Side.W_HN_Side_C|GetPageTotal (Variables|Default|GetSideUI)) (Utilities|Text|ToText(Integer) (Utilities|Array|Length (Variables|NoteSystem|GetNotes))))
              (Rendering|Components|TextRender|SetText (Variables|/Game/HorrorNotes/Widgets/W_HN_Side.W_HN_Side_C|GetPageNumber (Variables|Default|GetSideUI)) (Utilities|Text|ToText(Integer) (+ (Variables|Default|GetPages) 1)))
              (goto _label)))
          (:then_5
            (if (Variables|NoteSystem|GetPause%20Game?)
              (Game|SetGamePaused true))))
        (else
          (Game|SetGamePaused false)
          (CallFunction|RemoveWidget))))))

(fn ConstructionScript)
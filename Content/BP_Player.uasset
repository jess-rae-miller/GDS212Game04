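; BP_Player is the first-person player pawn that walks, looks around and interacts with objects in the world.
; It creates the MainUI widget on BeginPlay and maps input axes to movement and controller rotation.
; Each tick a short camera line trace finds an Interactable that allows interaction, stores it and toggles the interact prompt.
; Pressing Interact calls BeginInteraction on that stored target, passing it the UI.
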(event EventBeginPlay
  (bind _returnvalue (Game|ConstructObjectfromClass "/Game/MainUI.MainUI_C"))
  (UserInterface|Viewport|AddtoViewport _returnvalue 0)
  (Variables|Default|SetUI _returnvalue))

(event Collision|EventActorBeginOverlap
  (params (OtherActor :type Actor%20Object%20Reference)))

(event EventTick
  (params (DeltaSeconds :type Float%20%28single-precision%29))
  (bind _camera (Variables|Default|GetCamera))
  (bind _returnvalue (Transformation|GetWorldLocation _camera))
  (bind _outhit (Collision|LineTraceByChannel _returnvalue (+ _returnvalue (* (Math|Vector|GetForwardVector (Transformation|GetWorldRotation _camera)) 2.5e+02)) "TraceTypeQuery1" false 0 "None"))
  (bind _asinteractable (Utilities|Casting|CastToInteractable (.HitActor (Collision|BreakHitResult _outhit)))
    (:then
      (if (Variables|/Game/Interactable.Interactable_C|GetCanInteract _asinteractable)
        (Variables|Default|SetCurrentInteractable _asinteractable)
        (Default|ToggleInteractText (Variables|Default|GetUI) "Visible")
        (else
          (Variables|Default|SetCurrentInteractable 0 :!label _label)
          (Default|ToggleInteractText (Variables|Default|GetUI) "Hidden"))))
    (:CastFailed
      (goto _label))))

(event Input|ActionEvents|InputActionInteract
  (params (Key :type Key%20Structure))
  (bind _currentinteractable (Variables|Default|GetCurrentInteractable))
  (:Pressed
    (Utilities|IsValid _currentinteractable
      (:Is%20Valid
        (Default|BeginInteraction _currentinteractable (Variables|Default|GetUI))))))

(event Input|AxisEvents|InputAxisMoveForward/Backward
  (params (AxisValue :type Float%20%28single-precision%29))
  ;[1 1 1] Movement
  (Pawn|Input|AddMovementInput (Transformation|GetActorForwardVector) AxisValue false))

(event Input|AxisEvents|InputAxisMoveLeft/Right
  (params (AxisValue :type Float%20%28single-precision%29))
  ;[1 1 1] Movement
  (Pawn|Input|AddMovementInput (Transformation|GetActorRightVector) AxisValue false))

(event Input|AxisEvents|InputAxisLookLeft/Right
  (params (AxisValue :type Float%20%28single-precision%29))
  ;[1 1 1] Camera
  (Pawn|Input|AddControllerYawInput AxisValue))

(event Input|AxisEvents|InputAxisLookUp/Down
  (params (AxisValue :type Float%20%28single-precision%29))
  ;[1 1 1] Camera
  (Pawn|Input|AddControllerPitchInput AxisValue))

(fn ConstructionScript)